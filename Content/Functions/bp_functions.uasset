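; Function library for line-of-sight visibility, with helpers for radial tracing, procedural vision-cone meshes and debug printing.
; RayTracer sweeps line traces around an actor and returns actor-relative hit or end points; its fake-light mesh-building section is disconnected.
; SightToVertices turns sight points into triangle-fan vertices and indices, optionally closed for 360 degrees, and Make Cone creates a material-applied mesh section from such arrays.
; VisionTrace separately gathers unique components hit around a child actor.
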(fn Debugger
  (params (A :type String) (B :type String) (Condition :type Boolean))
  (if Condition
    (Development|PrintString 0 (Utilities|String|Append A B) true true "(R=0.000000,G=0.660000,B=1.000000,A=1.000000)" 0.0))
  (return))

(fn MakeCone
  (params (visionCone :type Procedural%20Mesh%20Component%20Object%20Reference) (mat_cone1 :type Material%20Interface%20Object%20Reference) (Vertices :type Array%20of%20Vectors) (Triangles :type Array%20of%20Integers))
  (LocalVariables|Setcone visionCone)
  (LocalVariables|Setmat_cone mat_cone1)
  (Class|ProceduralMeshComponent|CreateMeshSectionLinearColor (LocalVariables|Getcone) 0 Vertices Triangles 0 0 0 0 0 0 0 false)
  (Rendering|Material|SetMaterial (LocalVariables|Getcone) 0 (LocalVariables|Getmat_cone))
  (Transformation|SetWorldRotation (LocalVariables|Getcone) "0, 0, 0" false false)
  (return))

(fn SighttoVertices
  (params (v_sightPoints :type Array%20of%20Vectors) (v_verts :type Array%20of%20Vectors) (actor :type Actor%20Object%20Reference) (i_triangles :type Array%20of%20Integers) (360Deg :type Boolean))
  (bind _returnvalue (Transformation|GetActorLocation actor))
  (bind (_x _y) (Math|Vector|BreakVector _returnvalue))
  (LocalVariables|Setb_360 360Deg)
  (LocalVariables|Seti_tr i_triangles)
  (bind _output_get (LocalVariables|Setv_vrt v_verts))
  (Utilities|Array|SetArrayElem :TargetArray _output_get)
  (for (_array_element _array_index) v_sightPoints
    (Utilities|Array|SetArrayElem (LocalVariables|Getv_vrt) (+ _array_index 1) (Math|Vector|MakeVector (- (.X (Math|Vector|BreakVector _array_element)) _x) (- (.Y (Math|Vector|BreakVector _array_element)) _y) -1e+02)))
  (Utilities|Array|Resize (LocalVariables|Geti_tr) (* (Utilities|Array|Length (LocalVariables|Getv_vrt)) 3))
  (for _index (range 0 (* (Utilities|Array|Length (LocalVariables|Getv_vrt)) 3))
    (Utilities|Array|SetArrayElem (LocalVariables|Geti_tr) (* _index 3) 0)
    (Utilities|Array|SetArrayElem (LocalVariables|Geti_tr) (+ (* _index 3) 1) (+ _index 1))
    (Utilities|Array|SetArrayElem (LocalVariables|Geti_tr) (+ (+ (* _index 3) 1) 1) (+ (+ _index 1) 1)))
  (if (LocalVariables|Getb_360)
    (Utilities|Array|SetArrayElem (LocalVariables|Geti_tr) (- (Utilities|Array|Length (LocalVariables|Geti_tr)) 1) 1))
  (return (LocalVariables|Getv_vrt) (LocalVariables|Geti_tr)))

(fn RayTracer
  (params (verts :type Array%20of%20Vectors) (uv :type Array%20of%20Vector%202D%20Structures) (tr :type Array%20of%20Integers) (Target :type Actor%20Object%20Reference) (TraceChannel :type ETraceTypeQuery%20Enum :default "TraceTypeQuery1") (Radius :type Float%20%28single-precision%29) (nPolygons :type Integer) (mesh :type Procedural%20Mesh%20Component%20Object%20Reference) (lightColor1 :type Linear%20Color%20Structure))
  (LocalVariables|SetVertices verts)
  (LocalVariables|SetUVS uv)
  (LocalVariables|SetTriangles tr)
  (LocalVariables|Setchar Target)
  (LocalVariables|Settrace_channel TraceChannel)
  (LocalVariables|SetlightDistance Radius)
  (LocalVariables|Seti_nPolygons nPolygons)
  (LocalVariables|SetProceduralMesh mesh)
  (LocalVariables|SetlightColor lightColor1)
  (LocalVariables|Setlinetrace_angle (/ 3.6e+02 (Math|Conversions|ToFloat(Integer) (LocalVariables|Geti_nPolygons))))
  ;[1 1 1] Clear all arrays before repopulation them
  (Utilities|Array|Clear (LocalVariables|GetUVS))
  (Utilities|Array|Clear (LocalVariables|GetTriangles))
  (Utilities|Array|Clear (LocalVariables|GetVertices))
  ;[1 1 1] Add empty element
  (Utilities|Array|Add :TargetArray (LocalVariables|GetVertices))
  (Utilities|Array|Add :TargetArray (LocalVariables|GetUVS))
  ;[1 1 1] Line trace and return the length if hit or didnt
  (LocalVariables|Setv_endVector (* (Transformation|GetActorForwardVector (LocalVariables|Getchar)) (LocalVariables|GetlightDistance)))
  (for _index (range 0 (LocalVariables|Geti_nPolygons))
    (bind _output_get (LocalVariables|Setv_traceStart (+ (Transformation|GetActorLocation (LocalVariables|Getchar)) (LocalVariables|Getv_endVector))))
    (bind (_outhit _returnvalue) (Collision|LineTraceByChannel (LocalVariables|Getchar) (Transformation|GetActorLocation (LocalVariables|Getchar)) _output_get (LocalVariables|Gettrace_channel) true 0 "ForOneFrame"))
    (LocalVariables|Setb_traceHit _returnvalue)
    ;[1 1 1] Calculate the length from the player
    (LocalVariables|Setlinetrace_hitLoc (- (.Location (Collision|BreakHitResult _outhit)) (Transformation|GetActorLocation (LocalVariables|Getchar))))
    (LocalVariables|Setlinetrace_noHitLoc (- (.TraceEnd (Collision|BreakHitResult _outhit)) (Transformation|GetActorLocation (LocalVariables|Getchar))))
    (LocalVariables|Setv_endVector (Math|Vector|RotateVector (LocalVariables|Getv_endVector) (Math|Rotator|MakeRotator 0.0 0.0 (LocalVariables|Getlinetrace_angle))))
    (if (LocalVariables|Getb_traceHit)
      ;[1 1 1] If hit return the hit location
      (Utilities|Array|Add (LocalVariables|GetVertices) (LocalVariables|Getlinetrace_hitLoc))
      (Utilities|Array|Add (LocalVariables|GetUVS) (Math|Vector2D|MakeVector2D (Math|Float|MapRangeClamped (Math|Vector|VectorLength (LocalVariables|Getlinetrace_hitLoc)) 0.0 (LocalVariables|GetlightDistance) 0.0 1.0) (Math|Float|MapRangeClamped (Math|Vector|VectorLength (LocalVariables|Getlinetrace_hitLoc)) 0.0 (LocalVariables|GetlightDistance) 0.0 1.0)))
      (else
        ;[1 1 1] If didn't hit return the end of the trace
        (Utilities|Array|Add (LocalVariables|GetVertices) (LocalVariables|Getlinetrace_noHitLoc))
        (Utilities|Array|Add (LocalVariables|GetUVS) "(X=1.000000,Y=1.000000)"))))
  (return (LocalVariables|GetVertices)))

(fn InitProcMeshVertArray
  (params (WorldContextObject :type Object%20Object%20Reference)))

(fn VisionTrace
  (params (player :type Actor%20Object%20Reference) (los_comp :type Child%20Actor%20Component%20Object%20Reference) (radius :type Float%20%28single-precision%29) (n_points :type Integer))
  (LocalVariables|Setchar player)
  (LocalVariables|SetchildActor_los los_comp)
  (LocalVariables|Setf_angle (/ 3.6e+02 (Math|Conversions|ToFloat(Integer) n_points)))
  (LocalVariables|Setf_distance radius)
  (LocalVariables|Setv_endVec (* (Transformation|GetActorForwardVector (LocalVariables|Getchar)) (LocalVariables|Getf_distance)))
  (for _index (range 0 n_points)
    (bind (_outhit _returnvalue) (Collision|LineTraceByChannel (LocalVariables|Getchar) (Transformation|GetActorLocation (Variables|/Script/Engine.ChildActorComponent|GetChildActor (LocalVariables|GetchildActor_los))) (+ (Transformation|GetActorLocation (Variables|/Script/Engine.ChildActorComponent|GetChildActor (LocalVariables|GetchildActor_los))) (LocalVariables|Getv_endVec)) "TraceTypeQuery1" false 0 "ForOneFrame"))
    (LocalVariables|Setv_endVec (Math|Vector|RotateVector (LocalVariables|Getv_endVec) (Math|Rotator|MakeRotator 0.0 0.0 (LocalVariables|Getf_angle))))
    (if _returnvalue
      (LocalVariables|Sethit_comp (.HitComponent (Collision|BreakHitResult _outhit)))
      (Utilities|Array|AddUnique (LocalVariables|Getcomponent_array) (LocalVariables|Gethit_comp))))
  (return (LocalVariables|Getcomponent_array)))