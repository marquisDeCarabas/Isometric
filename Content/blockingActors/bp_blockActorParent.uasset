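; Parent Blueprint for blocking actors that can switch between opaque and translucent looks and toggle custom depth rendering.
; The construction script applies the configured mesh and scale, builds opaque and translucent dynamic material instances sharing one color, and starts opaque.
; Translucent opacity is preset to the final fade amount, so events simply swap whole materials.
; Older runtime opacity-fade logic is left unconnected.
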(event EventBeginPlay)

(event Collision|EventActorBeginOverlap
  (params (OtherActor :type Actor%20Object%20Reference)))

(event EventTick
  (params (DeltaSeconds :type Float%20%28single-precision%29)))

(event EventRenderDepth
  (Rendering|SetRenderCustomDepth (Variables|Default|GetStaticMesh) true))

(event EventUnRenderDepth
  (Rendering|SetRenderCustomDepth (Variables|Default|GetStaticMesh) false))

(event EventToOpaque
  (Rendering|Material|SetMaterial (Variables|Default|GetStaticMesh) 0 (Variables|Default|Getmat_opaque)))

(event EventToTrnslcnt
  (Rendering|Material|SetMaterial (Variables|Default|GetStaticMesh) 0 (Variables|Default|Getmat_translucent)))

(fn ConstructionScript
  (bind _staticmesh (Variables|Default|GetStaticMesh))
  (Components|StaticMesh|SetStaticMesh _staticmesh (Variables|Default|Getmesh))
  (Transformation|SetWorldScale3D _staticmesh (Variables|Default|Getv_scale))
  (bind _returnvalue (Rendering|Material|CreateDynamicMaterialInstance _staticmesh 0 "/Game/blockingActors/mat_opacityChange.mat_opacityChange" "None" :!class /Script/Engine.PrimitiveComponent))
  (bind _output_get (Variables|Default|Setmat_translucent _returnvalue))
  (Rendering|Material|SetScalarParameterValue _output_get "Opacity" (Variables|Visibility|Getf_finalFadeAmount) :!class /Script/Engine.MaterialInstanceDynamic)
  (Rendering|Material|SetVectorParameterValue (Variables|Default|Getmat_translucent) "Color" (Variables|Default|Getmat_color) :!class /Script/Engine.MaterialInstanceDynamic)
  (bind _returnvalue_2 (Rendering|Material|CreateDynamicMaterialInstance _staticmesh 0 "/Game/blockingActors/mat_opacityChangeOpaque.mat_opacityChangeOpaque" "None" :!class /Script/Engine.PrimitiveComponent))
  (bind _output_get_2 (Variables|Default|Setmat_opaque _returnvalue_2))
  (Rendering|Material|SetVectorParameterValue _output_get_2 "Color" (Variables|Default|Getmat_color) :!class /Script/Engine.MaterialInstanceDynamic)
  (Rendering|Material|SetMaterial (Variables|Default|GetStaticMesh) 0 (Variables|Default|Getmat_opaque)))