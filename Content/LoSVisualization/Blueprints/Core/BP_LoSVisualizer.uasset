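; Child actor that draws its parent's line-of-sight area as a flat procedural mesh fan.
; An EQS query generates arc points from the parent's radius and angle, read through an interface, with spacing derived from MeshResolution.
; Results become actor-relative vertices around a center, with triangles built once using 360-degree wrap.
; Each finished query updates the mesh, resets its world rotation to zero and starts the next query a frame later.
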(event Custom|VisualizeLoSQueryResults
  (params (QueryInstance :type Env%20Query%20Instance%20Blueprint%20Wrapper%20Object%20Reference) (QueryStatus :type EEnvQueryStatus%20Enum :default "Processing"))
  ;[0 1 1 0.5] Line of Sight Visualization
  (bind _resultlocations (AI|EQS|GetQueryResultsasLocations QueryInstance))
  (bind _vertices (LineOfSightVisualization|BuildVertexDatafromEQSQueryResults _resultlocations)) ; Converts the query results into usable data
  (if (Variables|RuntimeAllocation|GetInitialized?)
    (LineOfSightVisualization|UpdateProcMeshSection _vertices) ; Uses the new vertex data to update the proc mesh vertices
    (else
      (bind _triangles (LineOfSightVisualization|BuildTriangleDataforVertices _vertices true))
      (LineOfSightVisualization|InitializeProcMeshSection _vertices _triangles)
      (Variables|RuntimeAllocation|SetInitialized? true)))
  (Utilities|FlowControl|Delay 0.0) ; Waits for next frame before calling the update function
  (CallFunction|EventUpdateVisualization) ; Starts the next round of visualization construction
)

(event Custom|EventUpdateVisualization
  ;[0 1 1 0.5] Line of Sight Visualization
  (bind _returnvalue (AI|EQS|RunEQSQuery (Variables|Config|GetLoSPointsGeneratorQuery) (Actor|GetParentActor) "AllMatching")) ; Runs EQS query for generating LoS points
  (bind (_arcradius _arcangle) (Class|BPILoSVisualization|RetrieveVisionRangeParameters(Message) (Actor|GetParentActor))) ; Retrieves the parent actor's vision range parameters through interface
  (AI|EQS|SetNamedParam _returnvalue "ArcRadius" _arcradius) ; Sets custom parameter values for the query
  (AI|EQS|SetNamedParam _returnvalue "ArcAngle" _arcangle) ; Sets custom parameter values for the query
  (AI|EQS|SetNamedParam _returnvalue "SpaceBetweenPoints" (Variables|RuntimeAllocation|GetMaxSpaceBetweenArcPoints)) ; Sets custom parameter values for the query
  (EventDispatchers|BindEventtoOnQueryFinishedEvent _returnvalue (delegate Custom|VisualizeLoSQueryResults)) ; Asks to be notified when the query has finished execution
)

(event EventBeginPlay
  ;[0 1 0 0.5] Initialization Protocols
  (if (Utilities|DoesObjectImplementInterface (Actor|GetParentActor) (Variables|Interfaces|GetCommunicationInterface)) ; Checks if the parent actor implements the necessary interface
    (|SetProcMeshMaterial)
    (InitializationProtocols|InitializeProcMeshVerticesArray)
    (InitializationProtocols|InitializeProcMeshTrianglesArray)
    (InitializationProtocols|CalculateSpaceBetweenArcPoints)
    (CallFunction|EventUpdateVisualization)
    (else
      (Development|PrintString "Warning: LoSVisualization Interface not detected"))))

(fn ConstructionScript)

(fn BuildVertexDatafromEQSQueryResults
  (params (EQSQueryResults :type Array%20of%20Vectors))
  (bind _returnvalue (Transformation|GetActorLocation))
  (bind (_x _y) (Math|Vector|BreakVector _returnvalue))
  ;[0 1 1 0.5] Takes the EQS query results to build usable vertex data for the proc mesh
  (Utilities|Array|SetArrayElem :TargetArray (Variables|RuntimeAllocation|GetProcMeshVertices)) ; Sets the arc center vertex location
  (for (_array_element _array_index) EQSQueryResults ; Loops through the query results to calculate displacement relative to the actor's world location
    (Utilities|Array|SetArrayElem (Variables|RuntimeAllocation|GetProcMeshVertices) (+ _array_index 1) (Math|Vector|MakeVector (- (.X (Math|Vector|BreakVector _array_element)) _x) (- (.Y (Math|Vector|BreakVector _array_element)) _y) 0.0)) ; Stores the calculated vertex location for proc mesh
  )
  (return (Variables|RuntimeAllocation|GetProcMeshVertices)))

(fn UpdateProcMeshSection
  (params (Vertices :type Array%20of%20Vectors))
  (Class|ProceduralMeshComponent|UpdateMeshSectionLinearColor (Variables|Default|GetLoSVisualization) 0 Vertices)
  (Transformation|SetWorldRotation (Variables|Default|GetLoSVisualization) "0, 0, 0" false false) ; Ensures that the rotation matches the parent actor
  (return))

(fn CalculateSpaceBetweenArcPoints
  ;[0 1 0 0.5] Uses the arc length formula to calculate the max space between two adjacent points on the LoS arc
  (bind _arcradius (Class|BPILoSVisualization|RetrieveVisionRangeParameters(Message) (Actor|GetParentActor)))
  (Variables|RuntimeAllocation|SetMaxSpaceBetweenArcPoints (/ (Math|Float|MultiplybyPi (* 2.0 _arcradius (/ 1.0 (Variables|Config|GetMeshResolution)))) 3.6e+02))
  (return))

(fn InitializeProcMeshVerticesArray
  ;[0 1 0 0.5] Sets the default size of vertices array, used for creating procedural mesh section
  (bind _arcangle (Class|BPILoSVisualization|RetrieveVisionRangeParameters(Message) (Actor|GetParentActor)))
  (Utilities|Array|Resize (Variables|RuntimeAllocation|GetProcMeshVertices) (+ (Math|Float|Ceil (* _arcangle (Variables|Config|GetMeshResolution))) 2))
  (return))

(fn InitializeProcMeshTrianglesArray
  ;[0 1 0 0.5] Sets the default size of triangles array, used for creating procedural mesh section
  (Utilities|Array|Resize (Variables|RuntimeAllocation|GetProcMeshTriangles) (* (- (Utilities|Array|Length (Variables|RuntimeAllocation|GetProcMeshVertices)) 2) 3))
  (return))

(fn InitializeProcMeshSection
  (params (Vertices :type Array%20of%20Vectors) (Triangles :type Array%20of%20Integers))
  (Class|ProceduralMeshComponent|CreateMeshSectionLinearColor (Variables|Default|GetLoSVisualization) 0 Vertices Triangles 0 0 0 0 0 0 0 false)
  (Transformation|SetWorldRotation (Variables|Default|GetLoSVisualization) "0, 0, 0" false false) ; Ensures that the rotation matches the parent actor
  (return))

(fn BuildTriangleDataforVertices
  (params (Vertices :type Array%20of%20Vectors) (b_360 :type Boolean))
  ;[0 1 1 0.5] Builds triangle mapping data for vertices
  (Variables|Default|Setb_360 b_360)
  (for _index (range 0 (- (Utilities|Array|Length Vertices) 2))
    (Utilities|Array|SetArrayElem (Variables|RuntimeAllocation|GetProcMeshTriangles) (* _index 3) 0) ; Maps 1st vertex of triangle to index of location (center = always zero)
    (Utilities|Array|SetArrayElem (Variables|RuntimeAllocation|GetProcMeshTriangles) (+ (* _index 3) 1) (+ _index 1)) ; Maps 2nd vertex of triangle to index of location
    (Utilities|Array|SetArrayElem (Variables|RuntimeAllocation|GetProcMeshTriangles) (+ (* _index 3) 2) (+ _index 2)) ; Maps 3rd vertex of triangle to index of location
  )
  (if (Variables|Default|Getb_360)
    (Utilities|Array|SetArrayElem (Variables|RuntimeAllocation|GetProcMeshTriangles) (- (Utilities|Array|Length (Variables|RuntimeAllocation|GetProcMeshTriangles)) 1) 1))
  (return (Variables|RuntimeAllocation|GetProcMeshTriangles)))