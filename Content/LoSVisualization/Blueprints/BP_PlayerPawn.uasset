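; BP_PlayerPawn is the player pawn for the line-of-sight visualization, moving along fixed forward and lateral vectors and turning to face the mouse cursor.
; A looping timer at roughly 60 Hz traces under the cursor on the Camera channel and changes only the actor's yaw toward the hit point.
; It implements BPI_LoSVisualization to expose its vision radius and angle as arc parameters.
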(event Custom|UpdateActorRotation
  ;[0 1 1 0.5] Player Orientation
  (CallFunction|OrientTowardstheCursor))

(event EventBeginPlay
  ;[0 1 1 0.5] Player Orientation
  (Input|SetInputModeGameOnly (Game|GetPlayerController 0))
  (Utilities|Time|SetTimerbyEvent (delegate Custom|UpdateActorRotation) 0.016667 true))

(event Input|AxisEvents|InputAxisMoveForward
  (params (AxisValue :type Float%20%28single-precision%29))
  ;[0 1 1 0.5] Movement Logic
  (Pawn|Input|AddMovementInput (Variables|Config|GetForwardMovementUnitVector) AxisValue false))

(event Input|AxisEvents|InputAxisMoveRight
  (params (AxisValue :type Float%20%28single-precision%29))
  ;[0 1 1 0.5] Movement Logic
  (Pawn|Input|AddMovementInput (Variables|Config|GetLateralMovementUnitVector) AxisValue false))

(fn ConstructionScript)

(fn OrientTowardstheCursor
  (bind _returnvalue (Transformation|GetActorRotation))
  (bind (_roll _pitch) (Math|Rotator|BreakRotator _returnvalue))
  ;[0 1 1 0.5] Modifies the actor's rotation to face the mouse cursor direction
  (Transformation|SetActorRotation (Math|Rotator|MakeRotator _roll _pitch (.Yaw (Math|Rotator|BreakRotator (Math|Rotator|FindLookatRotation (Transformation|GetActorLocation) (.Location (Collision|BreakHitResult (.HitResult (Game|Player|GetHitResultUnderCursorbyChannel (Game|GetPlayerController 0) "TraceTypeQuery2" false)))))))))
  (return))

(fn RetrieveVisionRangeParameters
  ;[0 1 0.4 0.5] BPI_LoSVisualization interface function
  (return (Variables|Config|GetVisionRadius) (Variables|Config|GetVisionAngle)))