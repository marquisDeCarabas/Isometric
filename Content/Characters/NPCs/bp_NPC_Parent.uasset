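; Parent NPC Blueprint for a stealth-style vision cone that shows the NPC's alert state, with alert and bubble widgets and interactable overlap tracking.
; ConeMaker turns EQS result points into a procedural mesh cone, coloured by state through a dynamic material.
; Helpers line-trace those points for the player and map blackboard senses to states.
; The EQS launch, player tracing and behaviour-choice calls are unwired, and VisionTracing is empty.
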(event OnComponentBeginOverlap(Collision)
  (params (OverlappedComponent :type Primitive%20Component%20Object%20Reference) (OtherActor :type Actor%20Object%20Reference) (OtherComp :type Primitive%20Component%20Object%20Reference) (OtherBodyIndex :type Integer) (bFromSweep :type Boolean) (SweepResult :type Hit%20Result%20Structure%20%28by%20ref%29))
  (if (Utilities|DoesObjectImplementInterface OtherActor "/Game/Interfaces/i_interact.i_interact_C")
    (Variables|Default|Setactor_interaction OtherActor)))

(event OnComponentEndOverlap(Collision)
  (params (OverlappedComponent :type Primitive%20Component%20Object%20Reference) (OtherActor :type Actor%20Object%20Reference) (OtherComp :type Primitive%20Component%20Object%20Reference) (OtherBodyIndex :type Integer))
  (if (Utilities|DoesObjectImplementInterface OtherActor "/Game/Interfaces/i_interact.i_interact_C")
    (Variables|Default|Setactor_interaction 0)))

(event Custom|ConeMaker
  (params (QueryInstance :type Env%20Query%20Instance%20Blueprint%20Wrapper%20Object%20Reference) (QueryStatus :type EEnvQueryStatus%20Enum :default "Processing"))
  ;[1 1 1] Run EQS to get end points for the rays and create a vision cone using them
  ;;[0.4001 1 0.4094] Create the cone
  (bind _resultlocations (AI|EQS|GetQueryResultsasLocations QueryInstance))
  (bind _output_get (Variables|MainCone|Setv_sightPoints _resultlocations))
  (bind (_vertices _triangles) (CallFunction|SighttoVertices _output_get (Variables|MainCone|Getv_vertices) self (Variables|MainCone|Geti_triangles) false))
  (CallFunction|MakeCone (Variables|Default|GetvisionCone) "/Game/Characters/NPCs/coneMaterial/mat_visionCone.mat_visionCone" _vertices _triangles)
  (bind _returnvalue (Rendering|Material|CreateDynamicMaterialInstance (Variables|Default|GetvisionCone) 0 "/Game/Characters/NPCs/coneMaterial/mat_visionCone.mat_visionCone" "None" :!class /Script/Engine.PrimitiveComponent))
  (Variables|MainCone|Setmat_coneInstance _returnvalue)
  (CallFunction|VisionTracing)
  (CallFunction|BehaviourColors (Variables|Default|Getstates))
  (Rendering|Material|SetVectorParameterValue (Variables|MainCone|Getmat_coneInstance) "Color" (Variables|Default|Getcolor_visionCone) :!class /Script/Engine.MaterialInstanceDynamic)
  (Rendering|Material|SetScalarParameterValue (Variables|MainCone|Getmat_coneInstance) "Opacity" (Variables|MainCone|Gets_coneOpacity) :!class /Script/Engine.MaterialInstanceDynamic))

(event Custom|visionTracing
  ;[1 1 1] Vision Tracing and updating player seen and location on the blackboard
)

(event EventBeginPlay
  ;[1 1 1] Begin play - init
  (Utilities|Array|Resize (Variables|MainCone|Getv_vertices) 51)
  (Variables|Default|Setf_runSpeed (Variables|/Script/Engine.CharacterMovementComponent|GetMaxWalkSpeed (Variables|Character|GetCharacterMovement)))
  (Variables|Default|Setstates "NewEnumerator0")
  (bind _asw_alert (Utilities|Casting|CastTow_alert (UserInterface|GetUserWidgetObject (Variables|Default|Getwidget_alertness))))
  (Variables|Default|Setw_alert _asw_alert)
  (bind _asw_bubble (Utilities|Casting|CastTow_Bubble (UserInterface|GetUserWidgetObject (Variables|Default|Getwidget_bubble))))
  (Variables|Default|Setw_bubble _asw_bubble)
  (bind _asw_bubble_2 (Utilities|Casting|CastTow_Bubble (UserInterface|GetUserWidgetObject (Variables|Default|Getwidget_exclamation))))
  (Variables|Default|Setw_exclaim _asw_bubble_2))

(event EventTick
  (params (DeltaSeconds :type Float%20%28single-precision%29))
  (Utilities|FlowControl|Sequence
    (:then_0
      (CallFunction|Debugger "NPC State : " (Utilities|String|EnumtoString (Variables|Default|Getstates)) (Variables|Default|Getb_debug)))))

(fn ConstructionScript
  (Variables|MainCone|Setf_angleLOS (Variables|MainCone|Getf_angleLOS))
  (Variables|MainCone|Setf_radiusLOS (Variables|MainCone|Getf_radiusLOS)))

(fn ConvertSightPoints2Vectices
  (params (sightPoints :type Array%20of%20Vectors))
  (bind _returnvalue (Transformation|GetActorLocation))
  (bind _v_vertices (Variables|MainCone|Getv_vertices))
  (bind _returnvalue_2 (Utilities|Array|Length _v_vertices))
  (bind (_x _y) (Math|Vector|BreakVector _returnvalue))
  (bind _returnvalue_3 (* _returnvalue_2 3))
  (Utilities|Array|SetArrayElem :TargetArray (Variables|MainCone|Getv_vertices))
  (for (_array_element _array_index) sightPoints
    (Utilities|Array|SetArrayElem (Variables|MainCone|Getv_vertices) (+ _array_index 1) (Math|Vector|MakeVector (- (.X (Math|Vector|BreakVector _array_element)) _x) (- (.Y (Math|Vector|BreakVector _array_element)) _y) 0.0)))
  (Utilities|Array|Resize (Variables|MainCone|Geti_triangles) _returnvalue_3)
  (for _index (range 0 _returnvalue_3)
    (Utilities|Array|SetArrayElem (Variables|MainCone|Geti_triangles) (* _index 3) 0)
    (Utilities|Array|SetArrayElem (Variables|MainCone|Geti_triangles) (+ (* _index 3) 1) (+ _index 1))
    (Utilities|Array|SetArrayElem (Variables|MainCone|Geti_triangles) (+ (+ (* _index 3) 1) 1) (+ _index 2)))
  (return (Variables|MainCone|Getv_vertices) (Variables|MainCone|Geti_triangles)))

(fn MaketheCone
  (params (vetices :type Array%20of%20Vectors) (triangles :type Array%20of%20Integers))
  (bind _visioncone (Variables|Default|GetvisionCone))
  (bind _mat_cone (Variables|MainCone|Getmat_cone))
  (Class|ProceduralMeshComponent|CreateMeshSectionLinearColor _visioncone 0 vetices triangles 0 0 0 0 0 0 0 false)
  (Rendering|Material|SetMaterial _visioncone 0 _mat_cone)
  (bind _returnvalue (Rendering|Material|CreateDynamicMaterialInstance _visioncone 0 _mat_cone "" :!class /Script/Engine.PrimitiveComponent))
  (Variables|MainCone|Setmat_coneInstance _returnvalue)
  (Transformation|SetWorldRotation _visioncone "0, 0, 0" false false))

(fn FindPlayer
  (params (locs :type Array%20of%20Vectors))
  (for _array_element locs
    (bind _outhit (Collision|LineTraceByChannel (Transformation|GetActorLocation) _array_element "TraceTypeQuery3" false 0 "None" true "(R=1.000000,G=0.000000,B=0.000000,A=1.000000)" "(R=0.000000,G=1.000000,B=0.000000,A=1.000000)" 0.2))
    (if (== (.HitActor (Collision|BreakHitResult _outhit)) (Game|GetPlayerCharacter 0))
      (AI|Components|Blackboard|SetValueasVector (AI|GetBlackboard 0) (Utilities|Name|MakeLiteralName "lastSeen") (.Location (Collision|BreakHitResult _outhit)))
      (return true (.Location (Collision|BreakHitResult _outhit)))))
  (return false "0, 0, 0"))

(fn VisionCounter)

(fn BehaviourColors
  (params (state :type Byte))
  (Utilities|StateChanger state
    (:Idle
      (Variables|Default|Setcolor_visionCone "(R=0.095715,G=1.000000,B=0.095572,A=1.000000)"))
    (:Suspicious
      (Variables|Default|Setcolor_visionCone "(R=0.847663,G=1.000000,B=0.115015,A=1.000000)"))
    (:Reacting
      (Variables|Default|Setcolor_visionCone "(R=1.000000,G=0.133942,B=0.110066,A=1.000000)"))
    (:Searching
      (Variables|Default|Setcolor_visionCone "(R=1.000000,G=0.481658,B=0.000000,A=1.000000)")))
  (return))

(fn BehaviourChooser
  (bind _returnvalue (AI|GetBlackboard 0))
  (if (ScalableFloat|GetValueasBool _returnvalue (Utilities|Name|MakeLiteralName "sensed"))
    (if (ScalableFloat|GetValueasBool _returnvalue (Utilities|Name|MakeLiteralName "playerVisible"))
      (Variables|Default|Setstates "NewEnumerator2")
      (else
        (Variables|Default|Setstates "NewEnumerator1")))
    (AI|Components|Blackboard|SetValueasEnum _returnvalue (Utilities|Name|MakeLiteralName "state") (Variables|Default|Getstates))))

(fn RetrieveVisionRangeParameters
  (return (Variables|MainCone|Getf_radiusLOS) (Variables|MainCone|Getf_angleLOS)))